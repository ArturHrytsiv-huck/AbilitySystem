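; GA_FireBolt is a gameplay ability that casts a fire bolt projectile toward the point under the mouse.
; On activation it gets target data under the mouse and turns the avatar to face that location through CombatInterface.
; It plays the cast montage and waits for the montage's gameplay event before spawning the projectile at that target and ending the ability.
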(event Ability|EventActivateAbility
  (bind _datahandle (|TargetDataUnderMouse)
    (:ValidData
      (Variables|Default|SetProjectileTagetLocation (.Location (Collision|BreakHitResult (Ability|TargetData|GetHitResultfromTargetData _datahandle))))
      (bind _ascombat_interface (Utilities|Casting|CastToCombatInterface (Ability|GetAvatarActorfromActorInfo)))
      (Class|CombatInterface|UpdateFacingTarget _ascombat_interface (Variables|Default|GetProjectileTagetLocation))
      (|PlayMontageandWaitProxy "None" "/Game/_GAME/Blueprint/Character/Animations/Abilities/AM_CastFireBolt.AM_CastFireBolt" 1.0 "None" true 1.0 0.0 false
        (:then
          (Ability|Tasks|WaitGameplayEvent "(TagName=\"Event.Montage.FireBolt\")" 0
            (:EventReceived
              (Class|ASProjectileSpell|SpawnProjectile (Variables|Default|GetProjectileTagetLocation))
              (Ability|EndAbility))))))))